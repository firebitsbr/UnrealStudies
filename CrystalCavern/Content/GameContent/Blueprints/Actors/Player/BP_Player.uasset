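; BP_Player is the player actor in a crystal-collecting game, moved by rolling its mesh with torque.
; Two input axes apply movement-speed-scaled torque to PlayerMesh as acceleration, while AdjustCameraArm sets the camera arm's length and world pitch.
; BeginPlay fades the camera in, then prints the collect-all-crystals objective.
; Any damage counts as death, triggering a one-time fade to black and a reload of the current level.
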(event `self.ReceiveBeginPlay`
  ;[1 1 1] Begin Stage Logic
  (`PlayerCameraManager.StartCameraFade` :`self` (`GameplayStatics.GetPlayerCameraManager` 0) :`FromAlpha` 1.0 :`Duration` (`self.FadeInTime`))
  (`KismetSystemLibrary.Delay` (`self.FadeInTime`))
  (`KismetSystemLibrary.PrintString` "COLLECT ALL CRYSTALS BEFORE REACH THE END" true true (struct :`G` 1.0 :`B` 0.115849 :`A` 1.0)))

(event `InputAxis|Move Fowards/Backwards`
  (params (AxisValue :type "Float (single-precision)"))
  ;[1 1 1] Movement Controls Logic
  (`PrimitiveComponent.AddTorqueInRadians` (`self.PlayerMesh`) (`KismetMathLibrary.MakeVector` 0.0 (* AxisValue (`self.MovementSpeed`))) "None" true))

(event `InputAxis|Move Right/Left`
  (params (AxisValue :type "Float (single-precision)"))
  ;[1 1 1] Movement Controls Logic
  (`PrimitiveComponent.AddTorqueInRadians` (`self.PlayerMesh`) (`KismetMathLibrary.MakeVector` (* AxisValue (`self.MovementSpeed`))) "None" true))

(event `self.ReceiveAnyDamage`
  (params (Damage :type "Float (single-precision)") (DamageType :type "DamageType Object Reference") (InstigatedBy :type "Controller Object Reference") (DamageCauser :type "Actor Object Reference"))
  ;[1 1 1] Player Die Event
  (`/Engine/EditorBlueprintResources/StandardMacros.DoOnce` false
    (:`Completed`
      (`PlayerCameraManager.StartCameraFade` :`self` (`GameplayStatics.GetPlayerCameraManager` 0) :`ToAlpha` 1.0 :`Duration` 1.0 :`bHoldWhenFinished` true)
      (`KismetSystemLibrary.Delay` 1.0)
      (bind _returnvalue (`GameplayStatics.GetCurrentLevelName` true))
      (`GameplayStatics.OpenLevel` (`KismetStringLibrary.Conv_StringToName` _returnvalue)))))

(fn `AdjustCameraArm`
  (params (Distance :type "Float (double-precision)") (Angle :type "Float (double-precision)"))
  (bind _cameraarm (`self.CameraArm`))
  (set `SpringArmComponent.TargetArmLength` Distance _cameraarm)
  (`SceneComponent.K2_SetWorldRotation` _cameraarm (`KismetMathLibrary.MakeRotator` 0.0 Angle) false false))

(fn `UserConstructionScript`)