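; BP_GameWinTrigger is an overlap trigger that completes the level when the player enters it with no BP_Crystal actors left.
; If crystals remain, it damages the player instead.
; Otherwise it prints a success message and, after a short delay, opens the next level or quits on the last one.
; Level order comes from the Levels array, indexed by the current level's name.
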(event `self.ReceiveActorBeginOverlap`
  (params (OtherActor :type "Actor Object Reference"))
  (`/Game/GameContent/Blueprints/Libraries/CC_MacroLibrary.IsPlayer` OtherActor
    (:`IsPlayer`
      (if (`self.AnyCrystalsRemaining`)
        (`GameplayStatics.ApplyDamage` OtherActor 1.0)
        (else
          (`KismetSystemLibrary.PrintString` "COLLECTED ALL CRYSTALS!")
          (`KismetSystemLibrary.Delay` 2.0)
          (if (`self.IsLastevel`)
            (`KismetSystemLibrary.QuitGame` null "Quit")
            (else
              (`self.LoadNextLevel`))))))))

(fn `AnyCrystalsRemaining`
  (returns (ReturnValue :type Boolean))
  (bind _outactors (`GameplayStatics.GetAllActorsOfClass` "/Game/GameContent/Blueprints/Actors/Collectibles/BP_Crystal.BP_Crystal_C"))
  (return (!= (`KismetArrayLibrary.Array_Length` _outactors) 0)))

(fn `GetLevelIndex`
  (returns (Index :type Integer))
  (bind _returnvalue (`GameplayStatics.GetCurrentLevelName` true))
  (return (`KismetArrayLibrary.Array_Find` (`self.Levels`) (`KismetStringLibrary.Conv_StringToName` _returnvalue))))

(fn `IsLastevel`
  (returns (IsLast :type Boolean))
  (return (== (`self.GetLevelIndex`) (`KismetArrayLibrary.Array_LastIndex` (`self.Levels`)))))

(fn `LoadNextLevel`
  (`GameplayStatics.OpenLevel` (`|GetArrayItem` (`self.Levels`) (+ (`self.GetLevelIndex`) 1))))

(fn `UserConstructionScript`)