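; Ammo pickup actor that gives a marine a random amount of stored ammo.
; On BeginPlay it rolls its amount between a configurable minimum and maximum.
; On overlap with a BP_Marine whose ammo storage is not full, it adds that amount to the stored ammo and destroys itself; otherwise it stays in the world.
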(event `self.ReceiveBeginPlay`
  (`self.SetAmmoAmount`))

(event `self.ReceiveActorBeginOverlap`
  (params (OtherActor :type "Actor Object Reference"))
  (`self.RecoverAmmo` OtherActor))

(fn `RecoverAmmo`
  (params (Object :type "Object Object Reference"))
  (bind _asbp_marine (cast `/Game/Blueprints/Pawns/Player/BP_Marine` Object))
  (bind _returnvalue (`/Game/Blueprints/Pawns/Player/BP_Marine.IsAmmoStorageFull` _asbp_marine))
  (if (not _returnvalue)
    (bind _result (`/Engine/EditorBlueprintResources/StandardMacros.NegateInt` (`self.AmountAmmo`))
      (:`  `
        (`/Game/Blueprints/Pawns/Player/BP_Marine.UpdateStoredAmmo` _asbp_marine _result)
        (`self.K2_DestroyActor`)))))

(fn `SetAmmoAmount`
  (set `self.AmountAmmo` (`KismetMathLibrary.RandomIntegerInRange` (`self.MinAmmoPickup`) (`self.MaxAmmoPickup`))))

(fn `UserConstructionScript`)