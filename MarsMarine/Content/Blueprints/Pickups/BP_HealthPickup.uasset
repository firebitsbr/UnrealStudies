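; BP_HealthPickup is a pickup that restores health to a BP_Marine that overlaps it.
; On BeginPlay it rolls its recovery amount at random between MinRecovery and MaxRecovery.
; On overlap it casts the actor to BP_Marine and, only if health is not full, passes the amount to UpdateHealth and destroys itself.
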(event `self.ReceiveBeginPlay`
  (`self.SetHealthRecoveryValue`))

(event `self.ReceiveActorBeginOverlap`
  (params (OtherActor :type "Actor Object Reference"))
  (`self.RecoverHealth` OtherActor))

(fn `RecoverHealth`
  (params (Actor :type "Object Object Reference"))
  (bind _asbp_marine (cast `/Game/Blueprints/Pawns/Player/BP_Marine` Actor))
  (if (not (`/Game/Blueprints/Pawns/Player/BP_Marine.IsHealthFull` _asbp_marine))
    (`/Game/Blueprints/Pawns/Player/BP_Marine.UpdateHealth` _asbp_marine (`self.HealthRecoveryValue`))
    (`self.K2_DestroyActor`)))

(fn `SetHealthRecoveryValue`
  (set `self.HealthRecoveryValue` (`KismetMathLibrary.RandomFloatInRange` (`self.MinRecovery`) (`self.MaxRecovery`))))

(fn `UserConstructionScript`)