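; Mission boundary volume that kills a BP_Marine staying outside the playable area for too long.
; Begin and end overlaps toggle the marine's OutsidePlaybleArea flag, and exiting starts the Kill event's TimeToKill delay.
; KillPlayer then rechecks the flag and applies damage equal to max health if still outside.
; The single Delay is shared, so exits during a countdown do not start separate timers.
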(event `self.ReceiveActorBeginOverlap`
  (params (OtherActor :type "Actor Object Reference"))
  (bind _asbp_marine (cast `/Game/Blueprints/Pawns/Player/BP_Marine` OtherActor))
  (set `/Game/Blueprints/Pawns/Player/BP_Marine.OutsidePlaybleArea` false _asbp_marine))

(event `self.ReceiveActorEndOverlap`
  (params (OtherActor :type "Actor Object Reference"))
  (bind _asbp_marine (cast `/Game/Blueprints/Pawns/Player/BP_Marine` OtherActor))
  (set `/Game/Blueprints/Pawns/Player/BP_Marine.OutsidePlaybleArea` true _asbp_marine)
  (`self.Kill` _asbp_marine))

(event `Kill`
  (params (Player :type "/Game/Blueprints/Pawns/Player/BP_Marine Object Reference"))
  ;[1 1 1] Kill Logic to support MP
  (`KismetSystemLibrary.Delay` (`self.TimeToKill`))
  (`self.KillPlayer` Player))

(fn `KillPlayer`
  (params (Player :type "/Game/Blueprints/Pawns/Player/BP_Marine Object Reference"))
  (if (`/Game/Blueprints/Pawns/Player/BP_Marine.OutsidePlaybleArea` Player)
    (`GameplayStatics.ApplyDamage` Player (`/Game/Blueprints/Pawns/Player/BP_Marine.PlayerMaxHealth` Player))))

(fn `UserConstructionScript`)