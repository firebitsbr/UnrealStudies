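; BP_Alien is an enemy AI character that chases the BP_Marine player and attacks in melee.
; A repeating AIMoveTo drives pursuit, while Tick halts movement to play the attack montage, resuming afterward.
; DamagePlayer applies range-checked damage but is not called within these graphs.
; On death it disables collision, credits the Marine's kill, notifies the game mode, then after a delay randomly drops health or ammo and destroys itself.
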(event `self.ReceiveBeginPlay`
  ;[1 1 1] AIMovementToPlayer
  (`self.GetTargetReference`)
  (if (`self.IsAlive`) :!label _label
    (`|AIMoveTo` self (0.0 0.0 0.0) (`self.Player`)
      (:`OnSuccess`
        _)
      (:`OnFail`
        _))
    (`KismetSystemLibrary.Delay` 0.2)
    (goto _label)))

(event `self.ReceiveTick`
  (params (DeltaSeconds :type "Float (single-precision)"))
  ;[1 1 1] AI Attack Logic
  (`/Engine/EditorBlueprintResources/StandardMacros.IsValid` (`self.Player`)
    (:`Is Valid`
      (if (`self.CanAttack`)
        (`self.DeactivateAIMovement`)
        (`|PlayMontage` (`self.Mesh`) "/Game/Characters/Enemy_Great_Spider/Animations/AnimMtgBP_AlienAttack01.AnimMtgBP_AlienAttack01"
          (:`OnCompleted`
            (`ActorComponent.Activate` (`self.CharacterMovement`) false)))))))

(event `self.ReceiveAnyDamage`
  (params (Damage :type "Float (single-precision)") (DamageType :type "DamageType Object Reference") (InstigatedBy :type "Controller Object Reference") (DamageCauser :type "Actor Object Reference"))
  ;[1 1 1] Damage and Death Logic
  (if (`self.IsAlive`)
    (`self.DecreaseHealth` DamageCauser Damage)
    (if (not (`self.IsAlive`))
      (`self.KillAI`)
      (`KismetSystemLibrary.Delay` (`self.TimeToDisapear`))
      (`self.SpawnPickups`)
      (`self.K2_DestroyActor`))))

(fn `CanAttack`
  (returns (ReturnValue :type Boolean))
  (return (and (`/Game/Blueprints/Pawns/Player/BP_Marine.IsAlive` (`self.Player`)) (`self.IsWithinAttackRange`) (`self.IsAlive`) (not (`self.IsAttacking`)))))

(fn `DamagePlayer`
  (if (`self.IsWithinAttackRange`)
    (`GameplayStatics.ApplyDamage` (`GameplayStatics.GetPlayerPawn` 0) (`self.DamagePerHit`))))

(fn `DeactivateAIMovement`
  (bind _charactermovement (`self.CharacterMovement`))
  (`ActorComponent.Deactivate` _charactermovement)
  (`MovementComponent.StopMovementImmediately` _charactermovement))

(fn `DecreaseHealth`
  (params (Actor :type "Actor Object Reference") (Value :type "Float (double-precision)"))
  (set `self.DamageCauser` Actor)
  (set `self.Health` (`KismetMathLibrary.FClamp` (- (`self.Health`) Value) 0.0 (`self.MaxHealth`))))

(fn `GetTargetReference`
  (bind _asbp_marine (cast `/Game/Blueprints/Pawns/Player/BP_Marine` (`GameplayStatics.GetPlayerPawn` 0)))
  (set `self.Player` _asbp_marine))

(fn `IsAlive`
  (returns (ReturnValue :type Boolean))
  (return (> (`self.Health`) 0.0)))

(fn `IsAttacking`
  (returns (`Return Value` :type Boolean))
  (return (`AnimInstance.Montage_IsPlaying` (`SkeletalMeshComponent.GetAnimInstance` (`self.Mesh`)) "/Game/Characters/Enemy_Great_Spider/Animations/AnimMtgBP_AlienAttack01.AnimMtgBP_AlienAttack01")))

(fn `IsWithinAttackRange`
  (returns (ReturnValue :type Boolean))
  (return (<= (`self.GetDistanceTo` (`GameplayStatics.GetPlayerPawn` 0)) (`self.AttackRange`))))

(fn `KillAI`
  (`self.DeactivateAIMovement`)
  (`self.SetActorEnableCollision` false)
  (bind _asbp_marine (cast `/Game/Blueprints/Pawns/Player/BP_Marine` (`self.DamageCauser`)))
  (`/Game/Blueprints/Pawns/Player/BP_Marine.AddKillCount` _asbp_marine)
  (bind _asbp_default_game_mode (cast `/Game/Blueprints/GameMode/BP_DefaultGameMode` (`GameplayStatics.GetGameMode`)))
  (`/Game/Blueprints/GameMode/BP_DefaultGameMode.RegisterAlienDeath` _asbp_default_game_mode self))

(fn `SpawnPickups`
  (bind _returnvalue (`self.GetTransform` self))
  (if (< (`KismetMathLibrary.RandomIntegerInRange` 0 100) (`self.PickupSpawnRate`))
    (if (< (`KismetMathLibrary.RandomIntegerInRange` 0 10) 5)
      (`|SpawnActorFromClass` "/Game/Blueprints/Pickups/BP_HealthPickup.BP_HealthPickup_C" _returnvalue "Undefined" "OverrideRootScale" null null)
      (else
        (`|SpawnActorFromClass` "/Game/Blueprints/Pickups/BP_AmmoPickup.BP_AmmoPickup_C" _returnvalue "Undefined" "OverrideRootScale" null null)))))

(fn `UserConstructionScript`)