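; Player-controlled marine for a shooter, with world-axis movement, health, ammo and reloading, plus a HUD widget created on BeginPlay.
; Each Tick smoothly turns control rotation toward the thumbstick or mouse-velocity direction outside a deadzone, depending on the last key's device.
; Firing runs a looping timer of muzzle-socket line traces that spend ammo, apply damage and spawn impacts.
; Damage updates health, and death deactivates movement and blocks aiming and firing.
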(event `InputAxis|Move Forward`
  (params (AxisValue :type "Float (single-precision)"))
  ;[1 1 1] Movement Logic
  (`self.AddMovementInput` (1.0 0.0 0.0) AxisValue))

(event `InputAxis|Move Right`
  (params (AxisValue :type "Float (single-precision)"))
  ;[1 1 1] Movement Logic
  (`self.AddMovementInput` (0.0 1.0 0.0) AxisValue))

(event `Key|AnyKey`
  (params (Key :type "Key Structure"))
  ;[1 1 1] Determine if player is Using Gamepad
  (:`Pressed`
    (set `self.UsingGamepad` (`KismetInputLibrary.Key_IsGamepadKey` Key))))

(event `self.ReceiveTick`
  (params (DeltaSeconds :type "Float (single-precision)"))
  ;[1 1 1] Updating Aim Direction
  (`self.UpdatePlayerAim`))

(event `InputAction|FIreWeapon`
  (params (Key :type "Key Structure"))
  ;[1 1 1] FIre Logic
  (:`Pressed`
    (if (`self.CanFire`)
      (`self.StartFiringWeapon`)))
  (:`Released`
    (if (`self.CanFire`)
      (`self.StopFiringWeapon`))))

(event `self.ReceiveBeginPlay`
  (bind _returnvalue (`|CreateWidget` "/Game/UI/W_PlayerHUD.W_PlayerHUD_C" null self))
  (bind _output_get (set `self.HUD` _returnvalue))
  (`UserWidget.AddToViewport` _output_get 0)
  (`self.SetupPlayer`))

(event `self.ReceiveAnyDamage`
  (params (Damage :type "Float (single-precision)") (DamageType :type "DamageType Object Reference") (InstigatedBy :type "Controller Object Reference") (DamageCauser :type "Actor Object Reference"))
  ;[1 1 1] Get Damage Logic
  (bind _result (`/Engine/EditorBlueprintResources/StandardMacros.NegateFloat` Damage)
    (:`  `
      (`self.UpdateHealth` _result)
      (`self.PlayerDeath`))))

(event `InputAction|Reload`
  (params (Key :type "Key Structure"))
  ;[1 1 1] Reload Logic
  (:`Pressed`
    (`self.Reload`)))

(fn `AddKillCount`
  (set `self.PlayerKills` (+ (`self.PlayerKills`) 1)))

(fn `AimUsingGamepad`
  (if (and (`self.IsThumbstickAboveDeadzone`) (`self.IsAlive`))
    (`Controller.SetControlRotation` (`GameplayStatics.GetPlayerController` 0) (`self.GetNextControlRotationSmooth` (`self.GetInputAxisValue`) (`self.GetInputAxisValue`)))))

(fn `AimUsingMouse`
  (bind (_x _y) (`KismetMathLibrary.BreakVector2D` (`self.GetMouseVelocity`)))
  (if (and (`self.IsMouseAboveDeadzone`) (`self.IsAlive`))
    (`Controller.SetControlRotation` (`GameplayStatics.GetPlayerController` 0) (`self.GetNextControlRotationSmooth` _x _y))))

(fn `CanFire`
  (returns (ReturnValue :type Boolean))
  (return (and (`self.IsAlive`) (> (`self.Ammo`) 0))))

(fn `CanReload`
  (returns (ReturnValue :type Boolean))
  (return (and (< (`self.Ammo`) (`self.MaxLoadedAmmo`)) (> (`self.StoredAmmo`) 0))))

(fn `GetMouseVelocity`
  (returns (ReturnValue :type "Vector2D Structure"))
  (bind (_deltax _deltay) (`PlayerController.GetInputMouseDelta` (`GameplayStatics.GetPlayerController` 0)))
  (return (/ (`KismetMathLibrary.MakeVector2D` _deltax _deltay) (`GameplayStatics.GetWorldDeltaSeconds`))))

(fn `GetNextControlRotation`
  (params (Y :type "Float (double-precision)") (X :type "Float (double-precision)"))
  (returns (ReturnValue :type "Rotator Structure"))
  (return (`KismetMathLibrary.MakeRotator` 0.0 0.0 (`KismetMathLibrary.DegAtan2` Y X))))

(fn `GetNextControlRotationSmooth`
  (params (X :type "Float (double-precision)") (Y :type "Float (double-precision)"))
  (returns (ReturnValue :type "Rotator Structure"))
  (return (`KismetMathLibrary.RInterpTo` (`Controller.GetControlRotation` (`GameplayStatics.GetPlayerController` 0)) (`self.GetNextControlRotation` X Y) (`GameplayStatics.GetWorldDeltaSeconds`) (`self.MouseSmoothingStrengh`))))

(fn `GetSelectedMaterial`
  (returns (NewParam :type "MaterialInterface Object Reference"))
  (return (`|GetArrayItem` (`self.Materials`) (`self.SelectedIndex`))))

(fn `GetWeaponTraceEndLocation`
  (returns (ReturnValue :type "Vector Structure"))
  (return (+ (`self.GetWeaponTraceStartLocation`) (* (`KismetMathLibrary.GetForwardVector` (`self.GetControlRotation`)) (`self.RifleRange`)))))

(fn `GetWeaponTraceStartLocation`
  (returns (ReturnValue :type "Vector Structure"))
  (return (`SceneComponent.GetSocketLocation` (`self.Weapon`) "MuzzleFlashSocket")))

(fn `HasStoredAmmo`
  (returns (`Return Value` :type Boolean))
  (return (> (`self.StoredAmmo`) 0)))

(fn `IsAlive`
  (returns (`Return Value` :type Boolean))
  (return (> (`self.PlayerHealth`) 0.0)))

(fn `IsAmmoStorageFull`
  (returns (ReturnValue :type Boolean))
  (return (== (`self.MaxAmmo`) (`self.StoredAmmo`))))

(fn `IsHealthFull`
  (returns (`Return Value` :type Boolean))
  (return (== (`self.PlayerHealth`) (`self.PlayerMaxHealth`))))

(fn `IsMouseAboveDeadzone`
  (returns (`Return Value` :type Boolean))
  (return (> (`KismetMathLibrary.VSize2D` (`self.GetMouseVelocity`)) (`self.MouseDeadzone`))))

(fn `IsThumbstickAboveDeadzone`
  (returns (`Return Value` :type Boolean))
  (return (> (`KismetMathLibrary.VSize2D` (`KismetMathLibrary.MakeVector2D` (`self.GetInputAxisValue`) (`self.GetInputAxisValue`))) (`self.ThumbstickDeadzone`))))

(fn `PlayerDeath`
  (if (not (`self.IsAlive`))
    (`ActorComponent.Deactivate` (`self.CharacterMovement`))))

(fn `Reload`
  (locals (NeededAmmo :type Integer :default 0))
  (if (`self.CanReload`)
    (`GameplayStatics.SpawnSound2D` "/Game/Sounds/Weapon_AssaultRifle/Stereo/AssaultRifle_Reload_Stereo_Cue.AssaultRifle_Reload_Stereo_Cue" 1.0 1.0 0.0 null)
    (bind _output_get (set `local.NeededAmmo` (- (`self.MaxLoadedAmmo`) (`self.Ammo`))))
    (if (>= _output_get (`self.StoredAmmo`))
      (if (`self.HasStoredAmmo`)
        (`self.UpdateAmmo` (+ (`self.Ammo`) (`self.StoredAmmo`)))
        (`self.UpdateStoredAmmo` (`self.StoredAmmo`))
        (return))
      (else
        (`self.UpdateAmmo` (`self.MaxLoadedAmmo`))
        (`self.UpdateStoredAmmo` (`local.NeededAmmo`))
        (return)))))

(fn `SetupPlayer`
  (`PrimitiveComponent.SetMaterial` (`self.Mesh`) 0 (`self.GetSelectedMaterial`))
  (`self.UpdateHealth` 0.0))

(fn `SpawnImpactHit`
  (params (Value :type "Vector Structure"))
  (`GameplayStatics.SpawnEmitterAtLocation` "/Game/Effects/Weapons/Impacts/P_AssaultRifle_IH.P_AssaultRifle_IH" Value))

(fn `StartFiringWeapon`
  (`ActorComponent.Activate` (`self.P_AssaultRifle_MF`) true)
  (bind _returnvalue (`GameplayStatics.SpawnSound2D` "/Game/Sounds/Weapon_AssaultRifle/Stereo/SoundCue_Rifle.SoundCue_Rifle" 1.0 1.0 0.0 null))
  (set `self.FireSound` _returnvalue)
  (`self.WeaponTrace`)
  (`KismetSystemLibrary.K2_SetTimer` null "WeaponTrace" (`self.WeaponFireRate`) true))

(fn `StopFiringWeapon`
  (`ActorComponent.Deactivate` (`self.P_AssaultRifle_MF`))
  (`AudioComponent.Stop` (`self.FireSound`))
  (`KismetSystemLibrary.K2_ClearTimer` null "WeaponTrace")
  (`GameplayStatics.SpawnSound2D` "/Game/Sounds/Weapon_AssaultRifle/Stereo/SoundCue_RifleEnd.SoundCue_RifleEnd" 1.0 1.0 0.0 null))

(fn `UpdateAmmo`
  (params (Value :type Integer))
  (set `self.Ammo` (`KismetMathLibrary.Clamp` (+ Value (`self.Ammo`)) 0 (`self.MaxLoadedAmmo`))))

(fn `UpdateHealth`
  (params (Increment :type "Float (double-precision)"))
  (set `self.PlayerHealth` (`KismetMathLibrary.FClamp` (+ Increment (`self.PlayerHealth`)) 0.0 (`self.PlayerMaxHealth`)))
  (`/Game/UI/W_PlayerHUD.UpdateHealthBar` (`self.HUD`)))

(fn `UpdatePlayerAim`
  (if (`self.UsingGamepad`)
    (`self.AimUsingGamepad`)
    (else
      (`self.AimUsingMouse`))))

(fn `UpdateStoredAmmo`
  (params (Value :type Integer))
  (set `self.StoredAmmo` (- (`self.StoredAmmo`) Value)))

(fn `UserConstructionScript`)

(fn `WeaponTrace`
  (`self.UpdateAmmo` -1)
  (`|ExecutionSequence`
    (:`then_0`
      (if (== (`self.Ammo`) 0)
        (`self.StopFiringWeapon`)))
    (:`then_1`
      (bind _outhit (`KismetSystemLibrary.LineTraceSingle` (`self.GetWeaponTraceStartLocation`) (`self.GetWeaponTraceEndLocation`) "TraceTypeQuery1"))
      (bind (_bblockinghit _binitialoverlap _time _distance _location _impactpoint _normal _impactnormal _physmat _hitactor) (`GameplayStatics.BreakHitResult` _outhit))
      (if _bblockinghit
        (`self.SpawnImpactHit` _location)
        (`GameplayStatics.ApplyDamage` _hitactor (`self.DamagePerShot`) null self)))))