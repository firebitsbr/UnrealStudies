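; BP_Marine is the player marine, with world-axis movement and twin-stick-style aiming by gamepad or mouse.
; The last key pressed picks the aim mode each Tick: thumbstick angle sets control yaw directly, while mouse velocity steers it with smoothing, both past deadzones.
; Firing toggles a muzzle-flash particle and rifle sounds without using ammo.
; BeginPlay creates the HUD and applies the selected material; health updates refresh the HUD, and Reload is defined but uncalled here.
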(event `InputAxis|Move Forward`
  (params (AxisValue :type "Float (single-precision)"))
  ;[1 1 1] Movement Logic
  (`self.AddMovementInput` (1.0 0.0 0.0) AxisValue))

(event `InputAxis|Move Right`
  (params (AxisValue :type "Float (single-precision)"))
  ;[1 1 1] Movement Logic
  (`self.AddMovementInput` (0.0 1.0 0.0) AxisValue))

(event `Key|AnyKey`
  (params (Key :type "Key Structure"))
  ;[1 1 1] Determine if player is Using Gamepad
  (:`Pressed`
    (set `self.UsingGamepad` (`KismetInputLibrary.Key_IsGamepadKey` Key))))

(event `self.ReceiveTick`
  (params (DeltaSeconds :type "Float (single-precision)"))
  ;[1 1 1] Updating Aim Direction
  (`self.UpdatePlayerAim`))

(event `InputAction|FIreWeapon`
  (params (Key :type "Key Structure"))
  ;[1 1 1] FIre Logic
  (:`Pressed`
    (`self.StartFiringWeapon`))
  (:`Released`
    (`self.StopFiringWeapon`)))

(event `self.ReceiveBeginPlay`
  (bind _returnvalue (`|CreateWidget` "/Game/UI/W_PlayerHUD.W_PlayerHUD_C" null self))
  (bind _output_get (set `self.HUD` _returnvalue))
  (`UserWidget.AddToViewport` _output_get 0)
  (`self.SetupPlayer`))

(fn `AimUsingGamepad`
  (if (`self.IsThumbstickAboveDeadzone`)
    (`Controller.SetControlRotation` (`GameplayStatics.GetPlayerController` 0) (`self.GetNextControlRotation` (`self.GetInputAxisValue`) (`self.GetInputAxisValue`)))))

(fn `AimUsingMouse`
  (if (`self.IsMouseAboveDeadzone`)
    (`Controller.SetControlRotation` (`GameplayStatics.GetPlayerController` 0) (`self.GetNextControlRotationSmooth`))))

(fn `GetMouseVelocity`
  (returns (ReturnValue :type "Vector2D Structure"))
  (bind (_deltax _deltay) (`PlayerController.GetInputMouseDelta` (`GameplayStatics.GetPlayerController` 0)))
  (return (/ (`KismetMathLibrary.MakeVector2D` _deltax _deltay) (`GameplayStatics.GetWorldDeltaSeconds`))))

(fn `GetNextControlRotation`
  (params (Y :type "Float (double-precision)") (X :type "Float (double-precision)"))
  (returns (ReturnValue :type "Rotator Structure"))
  (return (`KismetMathLibrary.MakeRotator` 0.0 0.0 (`KismetMathLibrary.DegAtan2` Y X))))

(fn `GetNextControlRotationSmooth`
  (returns (ReturnValue :type "Rotator Structure"))
  (bind (_x _y) (`KismetMathLibrary.BreakVector2D` (`self.GetMouseVelocity`)))
  (return (`KismetMathLibrary.RInterpTo` (`Controller.GetControlRotation` (`GameplayStatics.GetPlayerController` 0)) (`self.GetNextControlRotation` _x _y) (`GameplayStatics.GetWorldDeltaSeconds`) (`self.MouseSmoothingStrengh`))))

(fn `GetSelectedMaterial`
  (returns (NewParam :type "MaterialInterface Object Reference"))
  (return (`|GetArrayItem` (`self.Materials`) (`self.SelectedIndex`))))

(fn `IsMouseAboveDeadzone`
  (returns (`Return Value` :type Boolean))
  (return (> (`KismetMathLibrary.VSize2D` (`self.GetMouseVelocity`)) (`self.MouseDeadzone`))))

(fn `IsThumbstickAboveDeadzone`
  (returns (`Return Value` :type Boolean))
  (return (> (`KismetMathLibrary.VSize2D` (`KismetMathLibrary.MakeVector2D` (`self.GetInputAxisValue`) (`self.GetInputAxisValue`))) (`self.ThumbstickDeadzone`))))

(fn `Reload`
  (locals (NeededAmmo :type Integer :default 0))
  (bind _output_get (set `local.NeededAmmo` (- (`self.MaxLoadedAmmo`) (`self.Ammo`))))
  (if (>= _output_get (`self.StoredAmmo`))
    (set `self.Ammo` (`self.MaxLoadedAmmo`))
    (set `self.StoredAmmo` (- (`self.StoredAmmo`) (`local.NeededAmmo`)))
    (return)
    (elif (> (`self.StoredAmmo`) 0)
      (set `self.Ammo` (+ (`self.Ammo`) (`self.StoredAmmo`)))
      (set `self.StoredAmmo` 0)
      (return))))

(fn `SetupPlayer`
  (`PrimitiveComponent.SetMaterial` (`self.Mesh`) 0 (`self.GetSelectedMaterial`))
  (`self.UpdateHealth` 0.0))

(fn `StartFiringWeapon`
  (`ActorComponent.Activate` (`self.P_AssaultRifle_MF`) true)
  (bind _returnvalue (`GameplayStatics.SpawnSound2D` "/Game/Sounds/Weapon_AssaultRifle/Stereo/SoundCue_Rifle.SoundCue_Rifle" 1.0 1.0 0.0 null))
  (set `self.FireSound` _returnvalue))

(fn `StopFiringWeapon`
  (`ActorComponent.Deactivate` (`self.P_AssaultRifle_MF`))
  (`AudioComponent.Stop` (`self.FireSound`))
  (`GameplayStatics.SpawnSound2D` "/Game/Sounds/Weapon_AssaultRifle/Stereo/SoundCue_RifleEnd.SoundCue_RifleEnd" 1.0 1.0 0.0 null))

(fn `UpdateHealth`
  (params (Increment :type "Float (double-precision)"))
  (set `self.PlayerHealth` (+ Increment (`self.PlayerHealth`)))
  (`/Game/UI/W_PlayerHUD.UpdateHealthBar` (`self.HUD`)))

(fn `UpdatePlayerAim`
  (if (`self.UsingGamepad`)
    (`self.AimUsingGamepad`)
    (else
      (`self.AimUsingMouse`))))

(fn `UserConstructionScript`)