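; Game mode that runs escalating waves of BP_Alien enemies, starting after a delay.
; A looping timer spawns aliens at randomly chosen TargetPoint actors in the level until the wave's quota is used up.
; RegisterAlienDeath removes aliens from the tracked list and ends the wave when none are alive or pending.
; After a short pause, the next wave gets a larger quota and a shorter spawn interval via a difficulty multiplier.
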(event `self.ReceiveBeginPlay`
  (`KismetSystemLibrary.Delay` (`self.StartGameDelay`))
  (`self.SetupNewWave`))

(event `SpawnWave`
  (`self.SpawnAlien`))

(event `EndWave`
  (`KismetSystemLibrary.Delay` 5.0)
  (`self.IncreaseWaveDificulty`)
  (`self.SetupNewWave`))

(fn `GetRandomSpawnPoint`
  (returns (`Return Value` :type "TargetPoint Object Reference"))
  (bind _outactors (`GameplayStatics.GetAllActorsOfClass` "/Script/Engine.TargetPoint"))
  (return (`|GetArrayItem` _outactors (`KismetMathLibrary.RandomIntegerInRange` 0 (`KismetArrayLibrary.Array_LastIndex` _outactors)))))

(fn `IncreaseWaveDificulty`
  (bind _output_get (set `self.MaxAliensInWave` (`KismetMathLibrary.FCeil` (* (`self.MaxAliensInWave`) (`self.DificultyMultiplier`)))))
  (set `self.AmountAliensToSpawn` _output_get)
  (set `self.SpawnFrequency` (/ (`self.SpawnFrequency`) (`self.DificultyMultiplier`))))

(fn `IsWaveCompleted`
  (returns (ReturnValue :type Boolean))
  (return (and (== (`KismetArrayLibrary.Array_Length` (`self.Aliens`)) 0) (== (`self.AmountAliensToSpawn`) 0))))

(fn `RegisterAlienDeath`
  (params (Alien :type "/Game/Blueprints/AI/BP_Alien Object Reference"))
  (`KismetArrayLibrary.Array_RemoveItem` (`self.Aliens`) Alien)
  (if (`self.IsWaveCompleted`)
    (`self.EndWave`)))

(fn `SetupNewWave`
  (set `self.CurrentWave` (+ (`self.CurrentWave`) 1))
  (`KismetSystemLibrary.K2_SetTimer` null "SpawnWave" (`self.SpawnFrequency`) true))

(fn `SpawnAlien`
  (if (> (`self.AmountAliensToSpawn`) 0)
    (bind _return_value (`self.GetRandomSpawnPoint`))
    (`/Engine/EditorBlueprintResources/StandardMacros.IsValid` _return_value
      (:`Is Valid`
        (bind _returnvalue (`|SpawnActorFromClass` "/Game/Blueprints/AI/BP_Alien.BP_Alien_C" (`self.GetTransform` _return_value) "Undefined" "OverrideRootScale" null null))
        (`/Engine/EditorBlueprintResources/StandardMacros.IsValid` _returnvalue
          (:`Is Valid`
            (`KismetArrayLibrary.Array_Add` (`self.Aliens`) _returnvalue)
            (`/Engine/EditorBlueprintResources/StandardMacros.DecrementInt` (`self.AmountAliensToSpawn`))))))
    (else
      (`KismetSystemLibrary.K2_ClearTimer` null "SpawnWave"))))

(fn `UserConstructionScript`)